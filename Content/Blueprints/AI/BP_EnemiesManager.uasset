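; BP_EnemiesManager is a manager Blueprint that spawns the starting enemies at spawner actors placed in the level.
; On BeginPlay it rebuilds its spawn point list from all BP_AISpawner actors, printing their names, then waits five seconds before spawning.
; It spawns BP_NPC actors round-robin across those points, ignoring collisions and incrementing the index before use, so the second spawner normally goes first.
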(event EventBeginPlay
  (CallFunction|ClearSpawnPoints)
  (CallFunction|FindSpawnPoints)
  (Utilities|FlowControl|Delay 5.0)
  (CallFunction|SpawnEnemies (Variables|Default|GetStart%20Enemies%20to%20Spawn)))

(event Collision|EventActorBeginOverlap
  (params (OtherActor :type Actor%20Object%20Reference)))

(event EventTick
  (params (DeltaSeconds :type Float%20%28single-precision%29)))

(fn ConstructionScript)

(fn FindSpawnPoints
  (bind _outactors (Actor|GetAllActorsOfClass "/Game/Blueprints/AI/BP_AISpawner.BP_AISpawner_C"))
  (for _array_element _outactors
    (Utilities|Array|Add (Variables|Default|GetEnemiesSpawner) _array_element))
  (for _array_element_2 (Variables|Default|GetEnemiesSpawner)
    (Development|PrintString (Utilities|GetDisplayName _array_element_2))))

(fn ClearSpawnPoints
  (if (not (Utilities|Array|IsEmpty (Variables|Default|GetEnemiesSpawner)))
    (Utilities|Array|Clear (Variables|Default|GetEnemiesSpawner))))

(fn SpawnEnemies
  (params (enemiesToSpawn :type Integer))
  (LocalVariables|Setindex 0)
  (for _index (range 0 (- enemiesToSpawn 1))
    (Math|Integer|IncrementInt (LocalVariables|Getindex)
      (:%20%20
        (if (> (LocalVariables|Getindex) (- (Utilities|Array|Length (Variables|Default|GetEnemiesSpawner)) 1))
          (LocalVariables|Setindex 0))
        (Game|SpawnActorfromClass "/Game/Blueprints/AI/BP_NPC.BP_NPC_C" (Transformation|GetActorTransform (Utilities|Array|Get(acopy) (Variables|Default|GetEnemiesSpawner) (LocalVariables|Getindex))) "AlwaysSpawn" "MultiplyWithRoot" 0 0)))))