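; BP_NpcController is an AI controller for NPCs that starts the BT_NPC behavior tree when it possesses a pawn.
; On possess it focuses on the first player pawn and casts it to BP_Character.
; If the cast succeeds, it writes that character to the blackboard as Player and the controlled pawn's current location as TestPos.
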(event EventBeginPlay)

(event EventTick
  (params (DeltaSeconds :type Float%20%28single-precision%29)))

(event EventPossess
  (params (PossessedPawn :type Pawn%20Object%20Reference))
  (bind _returnvalue (AI|GetBlackboard 0))
  (AI|RunBehaviorTree "/Game/Blueprints/AI/BT_NPC.BT_NPC")
  (AI|SetFocus (Game|Player|GetPlayerPawn 0))
  (bind _asbp_character (Utilities|Casting|CastToBP_Character (Game|Player|GetPlayerPawn 0)))
  (AI|Components|Blackboard|SetValueasObject _returnvalue (Utilities|Name|MakeLiteralName "Player") _asbp_character)
  (AI|Components|Blackboard|SetValueasVector _returnvalue (Utilities|Name|MakeLiteralName "TestPos") (Transformation|GetActorLocation (Pawn|GetControlledPawn))))

(fn ConstructionScript)