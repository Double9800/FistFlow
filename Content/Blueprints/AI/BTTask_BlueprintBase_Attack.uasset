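; Behavior tree task that tells an NPC to attack the player.
; On AI execution it looks up the pawn's BP_NpcCombatComponent and calls its AttackEvent with the actor from the Player blackboard key.
; It finishes successfully right after triggering the attack, without waiting for it to end.
; If the controller, pawn or component is invalid, the task never calls FinishExecute.
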(event EventReceiveExecuteAI
  (params (OwnerController :type AI%20Controller%20Object%20Reference) (ControlledPawn :type Pawn%20Object%20Reference))
  (CallFunction|NewFunction OwnerController ControlledPawn))

(fn NewFunction
  (params (Controller :type Actor%20Object%20Reference) (Pawn :type Actor%20Object%20Reference))
  (bind _returnvalue (Actor|GetComponentbyClass Pawn "/Game/Blueprints/AI/BP_NpcCombatComponent.BP_NpcCombatComponent_C"))
  (if (and (Utilities|IsValid Controller) (Utilities|IsValid Pawn))
    (Utilities|IsValid _returnvalue
      (:Is%20Valid
        (Default|AttackEvent _returnvalue (AI|BehaviorTree|GetBlackboardValueasActor (Variables|Default|GetPlayer)))
        (AI|BehaviorTree|FinishExecute true)))))