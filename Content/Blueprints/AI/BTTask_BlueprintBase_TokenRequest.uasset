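; Behavior tree task that requests a token for the AI-controlled pawn from the game instance.
; On AI execution it validates the controller and pawn, then calls TokenRequest on BP_GameInstance with the pawn.
; It finishes successfully right after the call without checking a result; failed validity checks or a failed cast never reach FinishExecute.
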(event EventReceiveExecuteAI
  (params (OwnerController :type AI%20Controller%20Object%20Reference) (ControlledPawn :type Pawn%20Object%20Reference))
  (CallFunction|RequestToken OwnerController ControlledPawn))

(fn RequestToken
  (params (Conroller :type Actor%20Object%20Reference) (pawn :type Actor%20Object%20Reference))
  (if (and (Utilities|IsValid Conroller) (Utilities|IsValid pawn))
    (bind _asbp_game_instance (Utilities|Casting|CastToBP_GameInstance (Game|GetGameInstance)))
    (Utilities|IsValid _asbp_game_instance
      (:Is%20Valid
        (Default|TokenRequest _asbp_game_instance pawn)
        (AI|BehaviorTree|FinishExecute true)))))