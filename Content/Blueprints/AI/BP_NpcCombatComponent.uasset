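; NPC combat component that runs melee attacks on the player and holds the NPC's combat state.
; AttackEvent plays a random attack montage while enabling the player's parry window and attack icon, then finishes the supplied attack task on completion.
; ApplyDamage, triggered externally, closes that window, finishes the task and sends damage through the BP_Hittable interface.
; SetCombatState mirrors the state to the AI Blackboard, with per-state debug text and mesh material swaps.
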(event Custom|AttackEvent
  (params (player :type Actor%20Object%20Reference) (task :type BT%20Task%20Blueprint%20Base%20Attack%20Object%20Reference))
  (Variables|Default|SetPlayer player)
  (Variables|Default|SetattackTask task)
  (Utilities|IsValid (Actor|GetComponentbyClass (Variables|Default|GetPlayer) "/Game/Blueprints/Player/BP_PlayerCombatComponent.BP_PlayerCombatComponent_C")
    (:Is%20Valid
      (Default|ActiveIconAttack (Actor|GetComponentbyClass (Variables|Default|GetPlayer) "/Game/Blueprints/Player/BP_PlayerCombatComponent.BP_PlayerCombatComponent_C") "SelfHitTestInvisible")
      (Development|PrintString "Attacco")
      (Default|SetCanParry (Actor|GetComponentbyClass (Variables|Default|GetPlayer) "/Game/Blueprints/Player/BP_PlayerCombatComponent.BP_PlayerCombatComponent_C") true)
      (Animation|Montage|PlayMontage (Actor|GetComponentbyClass (Components|GetOwner) "/Script/Engine.SkeletalMeshComponent") (.OutItem (Utilities|Array|Random (Utilities|Array|MakeArray "/Game/Characters/Mannequins/Anims/Unarmed/Attack/MM_Attack_01_Montage.MM_Attack_01_Montage" "/Game/Characters/Mannequins/Anims/Unarmed/Attack/MM_Attack_02_Montage.MM_Attack_02_Montage" "/Game/Characters/Mannequins/Anims/Unarmed/Attack/MM_ChargedAttack_Montage.MM_ChargedAttack_Montage")))
        (:OnCompleted
          (Default|ActiveIconAttack (Actor|GetComponentbyClass (Variables|Default|GetPlayer) "/Game/Blueprints/Player/BP_PlayerCombatComponent.BP_PlayerCombatComponent_C") "Hidden")
          (Default|SetCanParry (Actor|GetComponentbyClass (Variables|Default|GetPlayer) "/Game/Blueprints/Player/BP_PlayerCombatComponent.BP_PlayerCombatComponent_C") false)
          (Default|FinishExecuteListener (Variables|Default|GetattackTask)))))))

(event Custom|ApplyDamage
  (bind _player (Variables|Default|GetPlayer))
  (bind _returnvalue (Actor|GetComponentbyClass _player "/Game/Blueprints/Player/BP_PlayerCombatComponent.BP_PlayerCombatComponent_C"))
  (Utilities|IsValid _returnvalue
    (:Is%20Valid
      (Default|ActiveIconAttack _returnvalue "Hidden")
      (Default|SetCanParry _returnvalue false)
      (Default|FinishExecuteListener (Variables|Default|GetattackTask))
      (if (Utilities|DoesObjectImplementInterface (Variables|Default|GetPlayer) "/Game/Blueprints/Interface/BP_Hittable.BP_Hittable_C")
        (Class|BPHittable|Hit(Message) (Variables|Default|GetPlayer) (Variables|Default|GetDamage))
        (Development|PrintString "HIT")))))

(event EventBeginPlay
  (bind _asbp_game_instance (Utilities|Casting|CastToBP_GameInstance (Game|GetGameInstance)))
  (Variables|Default|SetAs%20BP%20Game%20Instance _asbp_game_instance))

(event EventTick
  (params (DeltaSeconds :type Float%20%28single-precision%29)))

(fn GetCombatState
  (return (Variables|Default|GetCombatState)))

(fn SetCombatState
  (params (State :type E_CombatState%20Enum :default "NewEnumerator0"))
  (bind _returnvalue (Components|GetOwner))
  (bind _returnvalue_2 (AI|GetAIController _returnvalue))
  (bind _returnvalue_3 (AI|GetBlackboard _returnvalue_2))
  (bind _output_get (Variables|Default|SetCombatState State))
  (Development|PrintString (Utilities|String|EnumtoString _output_get) true true (Utilities|Select :Index _output_get :NewEnumerator0 "(R=0.111972,G=0.662382,B=1.000000,A=1.000000)" :NewEnumerator2 "(R=1.000000,G=0.000000,B=0.000000,A=1.000000)" :NewEnumerator3 "(R=1.000000,G=0.857666,B=0.059588,A=1.000000)" :NewEnumerator5 "" :NewEnumerator6 ""))
  (Utilities|IsValid _returnvalue_3
    (:Is%20Valid
      (AI|Components|Blackboard|SetValueasEnum _returnvalue_3 (Utilities|Name|MakeLiteralName "CurrentCombatState") (Variables|Default|GetCombatState))
      (Rendering|Material|SetMaterial (Actor|GetComponentbyClass (Components|GetOwner) "/Script/Engine.SkeletalMeshComponent") 0 (Utilities|Select :Index (Variables|Default|GetCombatState) :NewEnumerator0 "/Engine/Tutorial/SubEditors/TutorialAssets/Character/TutorialTPP_Mat.TutorialTPP_Mat" :NewEnumerator2 "/DatasmithContent/Materials/AliasReference.AliasReference" :NewEnumerator3 "/AnimationSharing/AnimSharingBlue.AnimSharingBlue" :NewEnumerator5 "/MeshModelingToolsetExp/Materials/BakeRenderCaptureOutputMaterial.BakeRenderCaptureOutputMaterial" :NewEnumerator6 "/Engine/EngineDebugMaterials/M_GeoInsp_Clay.M_GeoInsp_Clay")))))