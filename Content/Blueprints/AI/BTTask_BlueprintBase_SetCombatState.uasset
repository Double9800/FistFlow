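; Behavior tree task that sets an NPC's combat state to a configurable value.
; On execute it writes that value to the CombatState blackboard key and passes it to the pawn's BP_NpcCombatComponent, keeping the two in step.
; It succeeds when the component exists, fails when it is missing (after the blackboard is already written), and calls FinishAbort if the controller or pawn is invalid.
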(event EventReceiveExecuteAI
  (params (OwnerController :type AI%20Controller%20Object%20Reference) (ControlledPawn :type Pawn%20Object%20Reference))
  (CallFunction|SettingFunction OwnerController ControlledPawn))

(fn SettingFunction
  (params (Object :type Object%20Object%20Reference) (Controlled%20Pawn :type Pawn%20Object%20Reference))
  (bind _returnvalue (Actor|GetComponentbyClass Controlled%20Pawn "/Game/Blueprints/AI/BP_NpcCombatComponent.BP_NpcCombatComponent_C"))
  (if (and (Utilities|IsValid Object) (Utilities|IsValid Controlled%20Pawn))
    (Class|BTFunctionLibrary|SetBlackboardValueasEnum (Variables|Default|GetCombatState) (Variables|Default|GetCombatStateToSetValue))
    (Utilities|IsValid _returnvalue
      (:Is%20Valid
        (Default|SetCombatState _returnvalue (Variables|Default|GetCombatStateToSetValue))
        (AI|BehaviorTree|FinishExecute true))
      (:Is%20Not%20Valid
        (AI|BehaviorTree|FinishExecute false)))
    (else
      (Class|BTTaskBlueprintBase|FinishAbort))))