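; Player combat component that handles fist, kick and head-bang attacks on NPCs, plus parries against the current attacker.
; Attack frees the GameInstance token and hides the HUD attack icon if the target is the attacking NPC, then sets its combat state and applies an impulse along its forward vector.
; Parry, when allowed, turns the player toward the attacker and fist-attacks.
; EnemyCheck sphere-traces pawns along the owner's view.
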(event EventBeginPlay
  (bind _asbp_game_instance (Utilities|Casting|CastToBP_GameInstance (Game|GetGameInstance)))
  (Variables|Default|SetAs%20BP%20Game%20Instance _asbp_game_instance))

(event EventTick
  (params (DeltaSeconds :type Float%20%28single-precision%29)))

(fn ActiveIconAttack
  (params (InVisibility :type ESlateVisibility%20Enum :default "Visible"))
  (bind _asbp_player_controller (Utilities|Casting|CastToBP_PlayerController (Game|GetPlayerController 0)))
  (Widget|SetVisibility (Variables|/Game/Blueprints/BP_HUD.BP_HUD_C|GetBP_IconAttack (Variables|/Game/Blueprints/BP_PlayerController.BP_PlayerController_C|GetHUD _asbp_player_controller)) InVisibility))

(fn Attack
  (params (attackType :type E_AttackType%20Enum :default "NewEnumerator0") (enemy :type Actor%20Object%20Reference))
  (LocalVariables|SetCombatComponent (Actor|GetComponentbyClass enemy "/Game/Blueprints/AI/BP_NpcCombatComponent.BP_NpcCombatComponent_C"))
  (if (== enemy (Default|GetAttackingNPC (Variables|Default|GetAs%20BP%20Game%20Instance)))
    (Default|FreeToken (Variables|Default|GetAs%20BP%20Game%20Instance))
    (Setting|SetCanParry false)
    (CallFunction|ActiveIconAttack "Hidden"))
  (Utilities|IsValid (LocalVariables|GetCombatComponent)
    (:Is%20Valid
      (Default|SetCombatState (LocalVariables|GetCombatComponent) "NewEnumerator5")
      (switch Utilities|FlowControl|Switch|SwitchonE_AttackType attackType
        (:NewEnumerator0
          (CallFunction|FistAttack enemy))
        (:NewEnumerator1
          (CallFunction|KickAttack enemy))
        (:NewEnumerator2
          (CallFunction|HeadAttack enemy))))))

(fn FistAttack
  (params (Target :type Actor%20Object%20Reference))
  (Development|PrintString "Fist")
  (CallFunction|AttackImpulse (Variables|knockback|GetFist%20Impulse%20Force) true (Actor|GetComponentbyClass Target "/Script/Engine.CharacterMovementComponent")))

(fn KickAttack
  (params (Target :type Actor%20Object%20Reference))
  (Development|PrintString "Kick")
  (CallFunction|AttackImpulse (Variables|knockback|GetKick%20Impuls%20Force) true (Actor|GetComponentbyClass Target "/Script/Engine.CharacterMovementComponent")))

(fn HeadAttack
  (params (Target :type Actor%20Object%20Reference))
  (Development|PrintString "Head")
  (CallFunction|AttackImpulse (Variables|knockback|GetHead%20Impulse%20Force) true (Actor|GetComponentbyClass Target "/Script/Engine.CharacterMovementComponent")))

(fn Parry
  (bind _returnvalue (Components|GetOwner))
  (bind _as_bp_game_instance (Variables|Default|GetAs%20BP%20Game%20Instance))
  (bind _attackingnpc (Default|GetAttackingNPC _as_bp_game_instance))
  (bind _returnvalue_2 (Transformation|GetActorLocation _returnvalue))
  (bind _returnvalue_3 (Transformation|GetActorLocation _attackingnpc))
  (if (Variables|Default|GetbcanParry)
    (Setting|SetCanParry false)
    (CallFunction|ActiveIconAttack "Hidden")
    (Pawn|SetControlRotation (Game|GetPlayerController 0) (Math|Rotator|FindLookatRotation (Math|Vector|MakeVector (.x _returnvalue_2) (.y _returnvalue_2) (.z _returnvalue_2)) (Math|Vector|MakeVector (.x _returnvalue_3) (.y _returnvalue_3) (.z _returnvalue_3))))
    (CallFunction|Attack "NewEnumerator0" _attackingnpc)))

(fn SetCanParry
  (params (bcanParry :type Boolean))
  (Variables|Default|SetbcanParry bcanParry))

(fn GetCanParry
  (return (Variables|Default|GetbcanParry)))

(fn AttackImpulse
  (params (impulseForce :type Float%20%28single-precision%29) (bVelocityChange :type Boolean) (Target :type Character%20Movement%20Component%20Object%20Reference))
  (Physics|AddImpulse Target (* (Transformation|GetActorForwardVector (Components|GetOwner Target)) impulseForce) bVelocityChange))

(fn EnemyCheck
  (params (Radius :type Float%20%28single-precision%29) (Distance%20check :type Float%20%28double-precision%29))
  (bind _returnvalue (Components|GetOwner))
  (bind (_outlocation _outrotation) (Actor|GetActorEyesViewPoint _returnvalue))
  (bind (_outhit _returnvalue_2) (Collision|SphereTraceForObjects _outlocation (+ _outlocation (* (Math|Vector|GetForwardVector _outrotation) Distance%20check)) Radius (Utilities|Array|MakeArray "ObjectTypeQuery3") false (Utilities|Array|MakeArray (Components|GetOwner)) "ForOneFrame"))
  (return _outhit _returnvalue_2))