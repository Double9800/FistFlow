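; BP_Character is the player character, handling movement, camera look and melee combat input.
; Enhanced Input events delegate grab, parry, dodge, run and fist, kick or head attacks to BPPlayerCombatComponent, with attacks firing only when its enemy check finds a target.
; Tick ramps gamepad look sensitivity toward per-axis targets while the stick passes a deadzone, resetting it otherwise, and prints max walk speed for debugging.
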(event Input|EnhancedActionEvents|EnhancedInputActionIA_Move
  (params (ActionValue :type Vector%202D%20Structure) (ElapsedSeconds :type Float%20%28double-precision%29) (TriggeredSeconds :type Float%20%28double-precision%29) (InputAction :type Input%20Action%20Object%20Reference :default "/Game/Input/IA/IA_Move.IA_Move"))
  (Pawn|Input|AddMovementInput (Transformation|GetActorForwardVector) (.y ActionValue) false)
  (Pawn|Input|AddMovementInput (Transformation|GetActorRightVector) (.x ActionValue) false))

(event Input|EnhancedActionEvents|EnhancedInputActionIA_Look
  (params (ActionValue :type Vector%202D%20Structure) (ElapsedSeconds :type Float%20%28double-precision%29) (TriggeredSeconds :type Float%20%28double-precision%29) (InputAction :type Input%20Action%20Object%20Reference :default "/Game/Input/IA/IA_Look.IA_Look"))
  (Pawn|Input|AddControllerYawInput (* (.x ActionValue) (Variables|Default|GetmouseSensibilityX)))
  (Pawn|Input|AddControllerPitchInput (* (* (.y ActionValue) (Variables|Default|Getmouse%20Sensibility%20Y)) -1.0)))

(event Input|EnhancedActionEvents|EnhancedInputActionIA_Parry
  (params (ActionValue :type Boolean) (ElapsedSeconds :type Float%20%28double-precision%29) (TriggeredSeconds :type Float%20%28double-precision%29) (InputAction :type Input%20Action%20Object%20Reference :default "/Game/Input/IA/IA_Parry.IA_Parry"))
  (:Started
    (Default|Parry (Variables|Default|GetBP_PlayerCombatComponent))))

(event Input|EnhancedActionEvents|EnhancedInputActionIA_Fist
  (params (ActionValue :type Boolean) (ElapsedSeconds :type Float%20%28double-precision%29) (TriggeredSeconds :type Float%20%28double-precision%29) (InputAction :type Input%20Action%20Object%20Reference :default "/Game/Input/IA/IA_Fist.IA_Fist"))
  (:Started
    (bind (_outhit _benemychecked) (Default|EnemyCheck (Variables|Default|GetBP_PlayerCombatComponent) 5e+01 3.5e+02))
    (if _benemychecked
      (Default|Attack (Variables|Default|GetBP_PlayerCombatComponent) "NewEnumerator0" (.HitActor (Collision|BreakHitResult _outhit))))))

(event Input|EnhancedActionEvents|EnhancedInputActionIA_Head
  (params (ActionValue :type Boolean) (ElapsedSeconds :type Float%20%28double-precision%29) (TriggeredSeconds :type Float%20%28double-precision%29) (InputAction :type Input%20Action%20Object%20Reference :default "/Game/Input/IA/IA_Head.IA_Head"))
  (:Started
    (bind (_outhit _benemychecked) (Default|EnemyCheck (Variables|Default|GetBP_PlayerCombatComponent) 5e+01 3.5e+02))
    (if _benemychecked
      (Default|Attack (Variables|Default|GetBP_PlayerCombatComponent) "NewEnumerator2" (.HitActor (Collision|BreakHitResult _outhit))))))

(event Input|EnhancedActionEvents|EnhancedInputActionIA_Grab
  (params (ActionValue :type Boolean) (ElapsedSeconds :type Float%20%28double-precision%29) (TriggeredSeconds :type Float%20%28double-precision%29) (InputAction :type Input%20Action%20Object%20Reference :default "/Game/Input/IA/IA_Grab.IA_Grab"))
  (:Started
    (Default|GrabEvent (Variables|Default|GetBP_PlayerCombatComponent) (Variables|Default|GetGrabPoint))))

(event Input|EnhancedActionEvents|EnhancedInputActionIA_Kick
  (params (ActionValue :type Boolean) (ElapsedSeconds :type Float%20%28double-precision%29) (TriggeredSeconds :type Float%20%28double-precision%29) (InputAction :type Input%20Action%20Object%20Reference :default "/Game/Input/IA/IA_Kick.IA_Kick"))
  (:Started
    (bind (_outhit _benemychecked) (Default|EnemyCheck (Variables|Default|GetBP_PlayerCombatComponent) 5e+01 3.5e+02))
    (if _benemychecked
      (Default|Attack (Variables|Default|GetBP_PlayerCombatComponent) "NewEnumerator1" (.HitActor (Collision|BreakHitResult _outhit))))))

(event Input|EnhancedActionEvents|EnhancedInputActionIA_PadLook
  (params (ActionValue :type Vector%202D%20Structure) (ElapsedSeconds :type Float%20%28double-precision%29) (TriggeredSeconds :type Float%20%28double-precision%29) (InputAction :type Input%20Action%20Object%20Reference :default "/Game/Input/IA/IA_PadLook.IA_PadLook"))
  (Pawn|Input|AddControllerYawInput (* (.x ActionValue) (Variables|Default|Getpad%20sensibility%20X)))
  (Pawn|Input|AddControllerPitchInput (* (.y ActionValue) (Variables|Default|Getpad%20sensibility%20Y))))

(event Input|EnhancedActionEvents|EnhancedInputActionIA_Run
  (params (ActionValue :type Boolean) (ElapsedSeconds :type Float%20%28double-precision%29) (TriggeredSeconds :type Float%20%28double-precision%29) (InputAction :type Input%20Action%20Object%20Reference :default "/Game/Input/IA/IA_Run.IA_Run"))
  (bind _bp_playercombatcomponent (Variables|Default|GetBP_PlayerCombatComponent))
  (:Triggered
    (Default|Run _bp_playercombatcomponent :!label _label))
  (:Ongoing
    (goto _label))
  (:Completed
    (Default|CanceledRun _bp_playercombatcomponent)))

(event Input|EnhancedActionEvents|EnhancedInputActionIA_Dodge
  (params (ActionValue :type Boolean) (ElapsedSeconds :type Float%20%28double-precision%29) (TriggeredSeconds :type Float%20%28double-precision%29) (InputAction :type Input%20Action%20Object%20Reference :default "/Game/Input/IA/IA_Dodge.IA_Dodge"))
  (:Started
    (Default|Dodge (Variables|Default|GetBP_PlayerCombatComponent) (Input|EnhancedActionValues|GetIA_Move))))

(event EventBeginPlay
  (bind _asbp_game_instance (Utilities|Casting|CastToBP_GameInstance (Game|GetGameInstance)))
  (Variables|Default|SetAs%20BP%20Game%20Instance _asbp_game_instance))

(event EventTick
  (params (DeltaSeconds :type Float%20%28single-precision%29))
  (bind _returnvalue (Input|EnhancedActionValues|GetIA_PadLook))
  (CallFunction|PrintUtility)
  (if (> (Math|Float|Absolute(Float) (.x _returnvalue)) 0.2)
    (Variables|Default|Setpad%20sensibility%20X (Math|Interpolation|FInterpTo (Variables|Default|Getpad%20sensibility%20X) (Variables|Default|Getpad%20sens%20target%20X) (Utilities|Time|GetWorldDeltaSeconds) (Variables|Default|GetInterp%20Speed%20pad%20sense)))
    (else
      (Variables|Default|Setpad%20sensibility%20X 1.0)))
  (if (> (Math|Float|Absolute(Float) (.y _returnvalue)) 0.2)
    (Variables|Default|Setpad%20sensibility%20Y (Math|Interpolation|FInterpTo (Variables|Default|Getpad%20sensibility%20Y) (Variables|Default|Getpad%20sens%20target%20Y) (Utilities|Time|GetWorldDeltaSeconds) (Variables|Default|GetInterp%20Speed%20pad%20sense)))
    (else
      (Variables|Default|Setpad%20sensibility%20Y 1.0))))

(fn ConstructionScript)

(fn PrintUtility
  (Development|PrintString (Utilities|String|ToString(Float) (Variables|/Script/Engine.CharacterMovementComponent|GetMaxWalkSpeed (Variables|Character|GetCharacterMovement))) true true "(R=1.000000,G=0.000000,B=0.794237,A=1.000000)" 0.0))