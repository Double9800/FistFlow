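; Player combat component that handles fist, kick and head attacks, parry, enemy grab-and-throw, sprint and dodge.
; Attacks snap the player onto the enemy, then apply impulse knockback; parry counters the game instance's attacking NPC, whose attack token is freed.
; Grab sphere-traces and attaches an NPC, then throws it as a ragdoll toward the aim point.
; Stamina-limited sprint interpolates walk speed and FOV on tick; dodge launches the character with a timed cooldown.
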(event Custom|JumpOnEnemy
  (params (TargetRelativeLocation :type Vector) (TargetRelativeRotation :type Rotator) (bEaseOut :type Boolean) (bEaseIn :type Boolean) (OverTime :type Float%20%28single-precision%29) (bForceShortestRotationPath :type Boolean) (Enemy :type Actor%20Object%20Reference) (Attack%20Type :type E_AttackType%20Enum :default "NewEnumerator0"))
  (Variables|Default|SetEnemy Enemy)
  (Components|MoveComponentTo (Actor|GetComponentbyClass (Components|GetOwner) "/Script/Engine.CapsuleComponent") TargetRelativeLocation TargetRelativeRotation bEaseOut bEaseIn OverTime bForceShortestRotationPath)
  (Pawn|SetControlRotation (Game|GetPlayerController 0) TargetRelativeRotation)
  (switch Utilities|FlowControl|Switch|SwitchonE_AttackType Attack%20Type
    (:NewEnumerator0
      (Attack|FistAttack (Variables|Default|Getenemy)))
    (:NewEnumerator1
      (Attack|KickAttack (Variables|Default|Getenemy)))
    (:NewEnumerator2
      (Attack|HeadAttack (Variables|Default|Getenemy)))))

(event EventBeginPlay
  (bind _returnvalue (Components|GetOwner))
  (bind _returnvalue_2 (Components|GetOwner))
  (bind _returnvalue_3 (Actor|GetComponentbyClass _returnvalue_2 "/Script/Engine.CameraComponent"))
  (bind _returnvalue_4 (Actor|GetComponentbyClass _returnvalue "/Script/Engine.CharacterMovementComponent"))
  (bind _asbp_game_instance (Utilities|Casting|CastToBP_GameInstance (Game|GetGameInstance)))
  (Variables|Default|SetAs%20BP%20Game%20Instance _asbp_game_instance)
  (Variables|run|SetcurrRunTime (Variables|run|GetmaxRunTime))
  (Variables|run|SetbcanRun true)
  (Utilities|IsValid _returnvalue_4
    (:Is%20Valid
      (Variables|Default|SetOwnerCharMovement _returnvalue_4))
    (:Is%20Not%20Valid
      _))
  (Utilities|IsValid _returnvalue_3
    (:Is%20Valid
      (Variables|Default|SetOwnerCameraComp _returnvalue_3)
      (Variables|run|SetInit%20Max%20Walk%20Speed (Variables|/Script/Engine.CharacterMovementComponent|GetMaxWalkSpeed (Variables|Default|GetOwnerCharMovement)))
      (Variables|run|SetInitField%20Of%20View (Variables|/Script/Engine.CameraComponent|GetFieldOfView (Variables|Default|GetOwnerCameraComp))))))

(event EventTick
  (params (DeltaSeconds :type Float%20%28single-precision%29))
  (run|UpdateRunValue 5.0))

(fn ActiveIconAttack
  (params (InVisibility :type ESlateVisibility%20Enum :default "Visible"))
  (bind _asbp_player_controller (Utilities|Casting|CastToBP_PlayerController (Game|GetPlayerController 0)))
  (Widget|SetVisibility (Variables|/Game/Blueprints/UI/BP_HUD.BP_HUD_C|GetBP_IconAttack (Variables|/Game/Blueprints/Player/BP_PlayerController.BP_PlayerController_C|GetHUD _asbp_player_controller)) InVisibility))

(fn Attack
  (params (attackType :type E_AttackType%20Enum :default "NewEnumerator0") (enemyf :type Actor%20Object%20Reference))
  (bind _returnvalue (Actor|GetComponentsByClass enemyf "/Script/Engine.CapsuleComponent"))
  (bind _output (Utilities|Array|Get(acopy) _returnvalue 1))
  (LocalVariables|SetCombatComponent (Actor|GetComponentbyClass enemyf "/Game/Blueprints/AI/BP_NpcCombatComponent.BP_NpcCombatComponent_C"))
  (if (== enemyf (Default|GetAttackingNPC (Variables|Default|GetAs%20BP%20Game%20Instance)))
    (Default|FreeToken (Variables|Default|GetAs%20BP%20Game%20Instance))
    (Setting|SetCanParry false)
    (Attack|ActiveIconAttack "Hidden"))
  (Utilities|IsValid (LocalVariables|GetCombatComponent)
    (:Is%20Valid
      (Default|SetCombatState (LocalVariables|GetCombatComponent) "NewEnumerator5")
      (CallFunction|JumponEnemy (Transformation|GetWorldLocation _output) (Transformation|GetWorldRotation _output) true false 0.1 true enemyf attackType))))

(fn FistAttack
  (params (Target :type Actor%20Object%20Reference))
  (Development|PrintString "Fist")
  (Attack|AttackImpulse(knockback) (Variables|knockback|GetFist%20Impulse%20Force) true (Actor|GetComponentbyClass Target "/Script/Engine.CharacterMovementComponent")))

(fn KickAttack
  (params (Target :type Actor%20Object%20Reference))
  (Development|PrintString "Kick")
  (Attack|AttackImpulse(knockback) (Variables|knockback|GetKick%20Impuls%20Force) true (Actor|GetComponentbyClass Target "/Script/Engine.CharacterMovementComponent")))

(fn HeadAttack
  (params (Target :type Actor%20Object%20Reference))
  (Development|PrintString "Head")
  (Attack|AttackImpulse(knockback) (Variables|knockback|GetHead%20Impulse%20Force) true (Actor|GetComponentbyClass Target "/Script/Engine.CharacterMovementComponent")))

(fn Parry
  (bind _returnvalue (Components|GetOwner))
  (bind _as_bp_game_instance (Variables|Default|GetAs%20BP%20Game%20Instance))
  (bind _attackingnpc (Default|GetAttackingNPC _as_bp_game_instance))
  (bind _returnvalue_2 (Transformation|GetActorLocation _returnvalue))
  (bind _returnvalue_3 (Transformation|GetActorLocation _attackingnpc))
  (if (Variables|parry|GetbcanParry)
    (Setting|SetCanParry false)
    (Attack|ActiveIconAttack "Hidden")
    (Pawn|SetControlRotation (Game|GetPlayerController 0) (Math|Rotator|FindLookatRotation (Math|Vector|MakeVector (.x _returnvalue_2) (.y _returnvalue_2) (.z _returnvalue_2)) (Math|Vector|MakeVector (.x _returnvalue_3) (.y _returnvalue_3) (.z _returnvalue_3))))
    (Attack|Attack "NewEnumerator0" _attackingnpc)))

(fn SetCanParry
  (params (bcanParry :type Boolean))
  (Variables|parry|SetbcanParry bcanParry))

(fn GetCanParry
  (return (Variables|parry|GetbcanParry)))

(fn AttackImpulse(knockback)
  (params (impulseForce :type Float%20%28single-precision%29) (bVelocityChange :type Boolean) (Target :type Character%20Movement%20Component%20Object%20Reference))
  (Components|Movement|StopMovementImmediately Target)
  (Physics|AddImpulse Target (* (Math|Vector|Normalize (- (Transformation|GetActorLocation (Components|GetOwner Target)) (Transformation|GetActorLocation (Game|GetPlayerCharacter 0)))) impulseForce) bVelocityChange))

(fn EnemyCheck
  (params (Radius :type Float%20%28single-precision%29) (Distance%20check :type Float%20%28double-precision%29))
  (bind _returnvalue (Components|GetOwner))
  (bind (_outlocation _outrotation) (Actor|GetActorEyesViewPoint _returnvalue))
  (bind (_outhit _returnvalue_2) (Collision|SphereTraceForObjects _outlocation (+ _outlocation (* (Math|Vector|GetForwardVector _outrotation) Distance%20check)) Radius (Utilities|Array|MakeArray "ObjectTypeQuery3") false (Utilities|Array|MakeArray (Components|GetOwner)) "ForOneFrame"))
  (return _outhit _returnvalue_2))

(fn GrabEvent
  (params (GrabPoint :type Scene%20Component%20Object%20Reference))
  (if (Variables|Grab|GetbcanGrab)
    (Utilities|IsValid (Variables|Grab|GetActorGrabbed)
      (:Is%20Not%20Valid
        (bind (_outhit _benemychecked) (CallFunction|EnemyCheck 25.0 2.5e+02))
        (if _benemychecked
          (bind _output_get (Variables|Grab|SetActorGrabbed (.HitActor (Collision|BreakHitResult _outhit))))
          (if (== _output_get (Default|GetAttackingNPC (Variables|Default|GetAs%20BP%20Game%20Instance)))
            (Default|FreeToken (Variables|Default|GetAs%20BP%20Game%20Instance)))
          (if (Utilities|IsValid (Actor|GetComponentbyClass (Variables|Grab|GetActorGrabbed) "/Game/Blueprints/AI/BP_NpcCombatComponent.BP_NpcCombatComponent_C"))
            (Default|SetCombatState (Actor|GetComponentbyClass (Variables|Grab|GetActorGrabbed) "/Game/Blueprints/AI/BP_NpcCombatComponent.BP_NpcCombatComponent_C") "NewEnumerator6")
            (bind _asbp_npc (Utilities|Casting|CastToBP_NPC (Variables|Grab|GetActorGrabbed)))
            (LocalVariables|SetNPC _asbp_npc)
            (Variables|/Game/Blueprints/AI/BP_NPC.BP_NPC_C|SethasGrabbed (LocalVariables|GetNPC) true)
            (Pawn|Components|CharacterMovement|SetMovementMode (Variables|/Script/Engine.Character|GetCharacterMovement (LocalVariables|GetNPC)) "MOVE_Walking" 0)
            (Collision|SetCollisionEnabled (Variables|/Script/Engine.Character|GetCapsuleComponent (LocalVariables|GetNPC)) "NoCollision")
            (Class|PrimitiveComponent|SetNotifyRigidBodyCollision (Variables|/Script/Engine.Character|GetMesh (LocalVariables|GetNPC)) true)
            (Transformation|SetActorScale3D (Variables|Grab|GetActorGrabbed) "0.700000,0.700000,0.700000")
            (Variables|Grab|SetbcanGrab false)
            (Transformation|AttachComponentToComponent (Variables|Grab|GetActorGrabbed) GrabPoint "None" "SnapToTarget" "SnapToTarget" "KeepWorld" true)))))
    (else
      (Grab|LaunchGrabObject (Variables|Grab|GetLaunch%20Force)))))

(fn LaunchGrabObject
  (params (launchForce :type Float%20%28single-precision%29))
  (bind _returnvalue (Components|GetOwner))
  (bind (_outlocation _outrotation) (Actor|GetActorEyesViewPoint _returnvalue))
  (Transformation|DetachFromActor (Variables|Grab|GetActorGrabbed) "KeepWorld" "KeepWorld" "KeepWorld")
  (bind _asbp_npc (Utilities|Casting|CastToBP_NPC (Variables|Grab|GetActorGrabbed)))
  (LocalVariables|SetNPC _asbp_npc)
  (Collision|SetCollisionEnabled (Variables|/Script/Engine.Character|GetMesh (LocalVariables|GetNPC)) "QueryAndPhysics")
  (Class|SkeletalMeshComponent|SetAllBodiesBelowSimulatePhysics (Variables|/Script/Engine.Character|GetMesh (LocalVariables|GetNPC)) (Utilities|Name|MakeLiteralName "pelvis") true true)
  (bind (_outhit _returnvalue_2) (Collision|LineTraceByChannel _outlocation (+ _outlocation (* (Math|Vector|GetForwardVector _outrotation) launchForce)) "TraceTypeQuery1" false (Utilities|Array|MakeArray (Variables|Grab|GetActorGrabbed)) "ForDuration"))
  (Physics|AddImpulse (Variables|/Script/Engine.Character|GetMesh (LocalVariables|GetNPC)) (Math|Vector|SelectVector (* (Math|Vector|Normalize (- (.impactpoint _outhit) (Transformation|GetActorLocation (Variables|Grab|GetActorGrabbed)))) (Variables|Grab|GetLaunch%20Force)) (* (Math|Vector|Normalize (- (.traceend _outhit) (Transformation|GetActorLocation (Variables|Grab|GetActorGrabbed)))) (Variables|Grab|GetLaunch%20Force)) _returnvalue_2) "pelvis" true)
  (Transformation|SetActorScale3D (Variables|Grab|GetActorGrabbed) "1.000000,1.000000,1.000000")
  (Variables|Grab|SetbcanGrab true)
  (Variables|Grab|SetActorGrabbed 0))

(fn Run
  (if (Variables|run|GetbcanRun)
    (bind _output_get (Variables|run|SetcurrRunTime (- (Variables|run|GetcurrRunTime) 1.0)))
    (if (<= _output_get 0.0)
      (Variables|run|SetbcanRun false)
      (bind _returnvalue (Utilities|Time|SetTimerbyFunctionName 0 "resetRun" (Variables|run|GetTimeToResetRunAfterZero)))
      (Variables|run|SetTimerHandler _returnvalue)
      (Variables|run|SetcurrRunTime 0.0)
      (Variables|run|SetrunFOVCopy (Variables|run|GetInitField%20Of%20View))
      (Variables|run|SetrunVelocityCopy (Variables|run|GetInit%20Max%20Walk%20Speed))
      (else
        (Variables|run|SetrunFOVCopy (Variables|run|GetrunFOV))
        (Variables|run|SetrunVelocityCopy (Variables|run|GetrunVelocity))
        (Components|Tick|SetComponentTickEnabled true)))))

(fn ResetRun
  (Variables|run|SetcurrRunTime (Variables|run|GetmaxRunTime))
  (Variables|run|SetbcanRun true)
  (if (Utilities|Time|IsValidTimerHandle (Variables|run|GetTimerHandler))
    (Utilities|Time|ClearandInvalidateTimerbyHandle (Variables|run|GetTimerHandler))))

(fn GetCurRunTime
  (return (Variables|run|GetcurrRunTime)))

(fn CanceledRun
  (Variables|run|SetrunFOVCopy (Variables|run|GetInitField%20Of%20View))
  (Variables|run|SetrunVelocityCopy (Variables|run|GetInit%20Max%20Walk%20Speed)))

(fn UpdateRunValue
  (params (InterpSpeed :type Float%20%28double-precision%29))
  (Variables|/Script/Engine.CharacterMovementComponent|SetMaxWalkSpeed (Variables|Default|GetOwnerCharMovement) (Math|Interpolation|FInterpTo (Variables|/Script/Engine.CharacterMovementComponent|GetMaxWalkSpeed (Variables|Default|GetOwnerCharMovement)) (Variables|run|GetrunVelocityCopy) (Utilities|Time|GetWorldDeltaSeconds) InterpSpeed))
  (Camera|SetFieldOfView (Variables|Default|GetOwnerCameraComp) (Math|Interpolation|FInterpTo (Variables|/Script/Engine.CameraComponent|GetFieldOfView (Variables|Default|GetOwnerCameraComp)) (Variables|run|GetrunFOVCopy) (Utilities|Time|GetWorldDeltaSeconds) InterpSpeed)))

(fn Dodge
  (params (inputAction :type Vector%202D%20Structure))
  (bind _returnvalue (Components|GetOwner))
  (bind _returnvalue_2 (Components|GetOwner))
  (bind _returnvalue_3 (Game|Player|GetPlayerPawn 0))
  (bind _dodgespeed (Variables|Dodge|GetdodgeSpeed))
  (bind _returnvalue_4 (Class|Pawn|GetLastMovementInputVector _returnvalue_3))
  (bind _returnvalue_5 (Class|KismetMathLibrary|NormalSafe2D inputAction 0.0))
  (bind _returnvalue_6 (Transformation|GetActorRightVector _returnvalue_2))
  (bind _returnvalue_7 (Transformation|GetActorForwardVector _returnvalue))
  (bind _returnvalue_8 (* _returnvalue_6 (.x _returnvalue_5)))
  (bind _returnvalue_9 (* _returnvalue_7 (.y _returnvalue_5)))
  (bind _returnvalue_10 (+ _returnvalue_8 _returnvalue_9))
  (bind _returnvalue_11 (Math|Vector2D|MakeVector2D (.x _returnvalue_10) (.y _returnvalue_10)))
  (bind _returnvalue_12 (Class|KismetMathLibrary|NormalSafe2D _returnvalue_11 0.0))
  (bind _returnvalue_13 (* _returnvalue_12 _dodgespeed))
  (if (Variables|Dodge|GetbcanDodge)
    (if (or (> (Math|Float|Absolute(Float) (.x _returnvalue_4)) 0.1) (> (Math|Float|Absolute(Float) (.y _returnvalue_4)) 0.1))
      (Character|LaunchCharacter (Game|GetPlayerCharacter 0) (Math|Vector|MakeVector (.x _returnvalue_13) (.y _returnvalue_13) 0.0) true false)
      (else
        (Character|LaunchCharacter (Game|GetPlayerCharacter 0) (* (Transformation|GetActorForwardVector (Components|GetOwner)) (* (Variables|Dodge|GetdodgeSpeed) -1.0)) true false)))
    (Variables|Dodge|SetbcanDodge false)
    (bind _returnvalue_14 (Utilities|Time|SetTimerbyFunctionName 0 "ResetDodge" (Variables|Dodge|GetResetTimerDodge)))
    (Variables|Dodge|SetDodgeTimer _returnvalue_14)))

(fn ResetDodge
  (Variables|Dodge|SetbcanDodge true)
  (Utilities|Time|ClearandInvalidateTimerbyHandle (Variables|Dodge|GetDodgeTimer)))