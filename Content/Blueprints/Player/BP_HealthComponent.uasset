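; Health component that tracks an actor's current health and handles its death, for NPCs and the player alike.
; Health starts at MaxHealth, and AddHealth applies signed changes, clamping only at zero before calling DeadFunction.
; DeadFunction disables the owner's AI controller tick, stops its movement and halts its brain logic.
; An owner without an AI controller is treated as the player and only prints a debug message.
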(event EventBeginPlay
  (Variables|Default|SetcurrHealth (Variables|Default|GetmaxHealth)))

(event EventTick
  (params (DeltaSeconds :type Float%20%28single-precision%29)))

(fn AddHealth
  (params (add :type Float%20%28double-precision%29))
  (bind _output_get (Variables|Default|SetcurrHealth (+ (Variables|Default|GetcurrHealth) add)))
  (if (<= _output_get 0.0)
    (Variables|Default|SetcurrHealth 0.0)
    (CallFunction|DeadFunction)))

(fn GetHealth
  (return (Variables|Default|GetcurrHealth)))

(fn DeadFunction
  (bind _output_get (LocalVariables|SetAIController (AI|GetAIController (Components|GetOwner))))
  (Utilities|IsValid _output_get
    (:Is%20Valid
      (Actor|Tick|SetActorTickEnabled (LocalVariables|GetAIController))
      (AI|Navigation|StopMovement (LocalVariables|GetAIController))
      (AI|Logic|StopLogic (Variables|/Script/AIModule.AIController|GetBrainComponent (LocalVariables|GetAIController)) "DEAD")
      (Development|PrintString "FunzioneMorteNPC"))
    (:Is%20Not%20Valid
      (Development|PrintString "PlayerFunzioneMorte"))))